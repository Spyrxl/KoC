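; BP_JumpyThingy is an experimental actor that periodically jolts its static mesh.
; Tick feeds a one-second Delay, so roughly once per second the mesh gets a large world rotation and a unit impulse along world X.
; Each pulse also prints a Counter variable for debugging, but the delta-time accumulation and threshold check meant to drive it are disconnected and never run.
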(event EventBeginPlay)

(event Collision|EventActorBeginOverlap
  (params (OtherActor :type Actor%20Object%20Reference)))

(event EventTick
  (params (DeltaSeconds :type Float%20%28single-precision%29))
  (Utilities|FlowControl|Delay 1.0)
  (Transformation|AddWorldRotation (Variables|Default|GetStaticMesh) "0,0.000000,1000.000000" false false)
  (Physics|AddImpulse (Variables|Default|GetStaticMesh) (Math|Rotator|GetRotationXVector "0, 0, 0") "None" false)
  (Development|PrintString (Utilities|String|ToString(Float) (stale _output_get))))

(fn ConstructionScript)